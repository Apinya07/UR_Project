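; BP_PuzzelDoor is a puzzle door that swings open once enough items have been collected.
; A collect event increments the item count, and a separate check event compares it to the required maximum.
; When the threshold is met, a DoOnce triggers the open event, where a timeline interpolates the door's relative yaw to its open angle.
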(event Custom|open%20dorr
  (bind _door_rotation (Timeline|Open%20Door%20Anim Play)
    (:Update
      (Transformation|SetRelativeRotation (Variables|Default|GetDoor) (Math|Rotator|MakeRotator 0.0 0.0 (Math|Float|Lerp 0.0 1.2e+02 _door_rotation)) false false))))

(event Custom|Colleck%20Item
  (Math|Integer|IncrementInt (Variables|Default|GetCurrentItemsCollected)))

(event Custom|Opendor%20Check
  (if (>= (Variables|Default|GetCurrentItemsCollected) (Variables|Default|GetMaxItem%20Colleck))
    (Utilities|FlowControl|DoOnce false
      (:Completed
        (CallFunction|OpenDorr)))))

(event Collision|EventActorBeginOverlap
  (params (OtherActor :type Actor%20Object%20Reference)))

(event EventTick
  (params (DeltaSeconds :type Float%20%28single-precision%29)))

(fn ConstructionScript)